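; Performance stress-test actor that fills the scene with many individual static mesh components, not instanced meshes, and keeps them moving.
; The construction script raises the actor by half the instance count, then spreads NbInstances meshes evenly around a circle of Radius.
; Each mesh gets a random height, an angle-based rotation and a random uniform scale.
; Tick applies a small fixed local rotation to the whole actor, independent of delta time.
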(event `self.ReceiveBeginPlay`)

(event `self.ReceiveTick`
  (params (DeltaSeconds :type "Float (single-precision)"))
  (`self.K2_AddActorLocalRotation` (struct :`Yaw` 0.1)))

(fn `UserConstructionScript`
  (locals (angle :type "Float (double-precision)") (increment :type "Float (double-precision)"))
  (bind _angle (`local.angle`))
  (bind _returnvalue (`KismetMathLibrary.Conv_IntToDouble` (/ (`self.nbInstances`) 2)))
  ;[0 0 0] 2000 instances 30 fps
  ;[0 0 0] offset de l'actor
  (`self.K2_SetActorLocation` (`KismetMathLibrary.MakeVector` 0.0 0.0 (`KismetMathLibrary.Conv_IntToDouble` (/ (`self.nbInstances`) 2))))
  (set `local.increment` (/ 360.0 (`KismetMathLibrary.Conv_IntToDouble` (`self.nbInstances`))))
  (for _index (range (`self.nbInstances`))
    (bind _returnvalue_2 (`AddComponent|NODE_AddStaticMeshComponent-0` :`RelativeTransform` (`KismetMathLibrary.MakeTransform` (0.0 0.0 0.0) (struct))))
    (set `self.currentStaticMesh` _returnvalue_2)
    ;[0 0 0] Location
    (set `local.angle` (* _index (`local.increment`)))
    (`SceneComponent.K2_SetRelativeLocation` (`self.currentStaticMesh`) (`KismetMathLibrary.MakeVector` (* (`KismetMathLibrary.DegCos` _angle) (`self.radius`)) (* (`KismetMathLibrary.DegSin` _angle) (`self.radius`)) (`KismetMathLibrary.RandomFloatInRange` (* _returnvalue -1.0) _returnvalue)) false false)
    ;[0 0 0] rotation
    (`SceneComponent.K2_AddRelativeRotation` (`self.currentStaticMesh`) (`KismetMathLibrary.MakeRotator` 90.0 0.0 (+ (`local.angle`) 90.0)) false false)
    ;[0 0 0] scale
    (`SceneComponent.SetRelativeScale3D` (`self.currentStaticMesh`) (* (`KismetMathLibrary.MakeVector` 1.0 1.0 1.0) (+ (* (`KismetMathLibrary.RandomFloat`) 3.0) 1.0)))))