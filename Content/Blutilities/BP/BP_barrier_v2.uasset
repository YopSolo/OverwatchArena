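; BP_barrier_v2 is a spline-driven Blueprint that builds a row of plastic barriers with alternating colors.
; Its construction script adds a static mesh component at each spline point, using that point's local transform with yaw offset 90 degrees.
; Each mesh gets its own dynamic instance of M_PlasticBarrier, with BaseColor switching between two color variables on even and odd indices.
; The event graph contains no active logic.
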(fn `UserConstructionScript`
  (for _index (range (`SplineComponent.GetNumberOfSplinePoints` (`self.Spline`)))
    (bind _returnvalue (`SplineComponent.GetTransformAtSplinePoint` (`self.Spline`) _index "Local" false))
    (bind _returnvalue_2 (`AddComponent|NODE_AddStaticMeshComponent-0` :`RelativeTransform` (`KismetMathLibrary.MakeTransform` (.location _returnvalue) (`KismetMathLibrary.MakeRotator` (.roll (.rotation _returnvalue)) (.pitch (.rotation _returnvalue)) (+ (.yaw (.rotation _returnvalue)) 90.0)) (.scale _returnvalue))))
    (bind _returnvalue_3 (`KismetMaterialLibrary.CreateDynamicMaterialInstance` "/Game/Blutilities/TextureAndMaterials/M_PlasticBarrier.M_PlasticBarrier"))
    (`MaterialInstanceDynamic.SetVectorParameterValue` _returnvalue_3 "BaseColor" (`KismetMathLibrary.SelectColor` (`self.BarrierBaseColor_1`) (`self.BarrierBaseColor_2`) (== (mod _index 2) 0)))
    (`PrimitiveComponent.SetMaterial` _returnvalue_2 0 _returnvalue_3)))