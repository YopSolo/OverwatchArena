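; BP_GeneratedDynMeshActor_v2 is a Geometry Script generated dynamic mesh actor that builds a tessellated, texture-displaced version of a source static mesh.
; On rebuild it copies StaticMeshSource into the dynamic mesh, applies PN tessellation at TessellationLevel, displaces it from a texture map and recomputes normals.
; BakeToStaticMesh writes the resulting dynamic mesh into the StaticMeshTarget asset when one is set.
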(event `self.OnRebuildGeneratedMesh`
  (params (TargetMesh :type "DynamicMesh Object Reference"))
  (bind _staticmeshsource (`self.staticMeshSource`)
    (:`then`
      (bind _returnvalue (`GeometryScriptLibrary_StaticMeshFunctions.CopyMeshFromStaticMesh` _staticmeshsource TargetMesh (struct) (struct) null)
        (:`Success`
          (bind _returnvalue_2 (`GeometryScriptLibrary_MeshSubdivideFunctions.ApplyPNTessellation` _returnvalue (struct) (`self.Tessellation Level`) null))
          (bind _returnvalue_3 (`GeometryScriptLibrary_MeshDeformFunctions.ApplyDisplaceFromTextureMap` _returnvalue_2 (`self.Texture`) (make `GeometryScriptDisplaceFromTextureOptions` 10.0) 0 null))
          (`GeometryScriptLibrary_MeshNormalsFunctions.RecomputeNormals` _returnvalue_3 (struct) null))))
    (:`else`)))

(fn `bakeToStaticMesh`
  (bind _staticmeshtarget (`self.StaticMeshTarget`)
    (:`then`
      (bind _returnvalue (`BaseDynamicMeshComponent.GetDynamicMesh` (`self.DynamicMeshComponent`)))
      (`GeometryScriptLibrary_StaticMeshFunctions.CopyMeshToStaticMesh` _returnvalue _staticmeshtarget (struct) (struct) null))
    (:`else`)))

(fn `UserConstructionScript`)