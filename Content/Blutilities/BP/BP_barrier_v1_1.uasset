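; BP_barrier_v1_1 is a procedural barrier actor that builds a straight row of static mesh pieces.
; Its Construction Script adds Longueur mesh components along the local Y axis, offset by Spacing.
; Each piece randomly takes StaticMesh1 or StaticMesh2 through an unseeded RandomBool, so the mix can change on every reconstruction.
; The Event Graph holds only disabled placeholder events.
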(fn `UserConstructionScript`
  (for _index (range (`self.Longueur`))
    (bind _returnvalue (`AddComponent|NODE_AddStaticMeshComponent-0` :`RelativeTransform` (`KismetMathLibrary.MakeTransform` (`KismetMathLibrary.MakeVector` 0.0 (`KismetMathLibrary.Conv_IntToDouble` (* _index (`self.Spacing`)))))))
    (`StaticMeshComponent.SetStaticMesh` _returnvalue (select `bool` (`KismetMathLibrary.RandomBool`) :`false` (`self.StaticMesh_1`) :`true` (`self.StaticMesh_2`)))))