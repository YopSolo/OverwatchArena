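; BP_Spline_displacement is an actor pairing a Spline with a Niagara effect whose spawn rate is exposed through CustomSpawnRate.
; The construction script pushes that value into the Niagara UserSpawnRate parameter, and BeginPlay runs the "show splines" console command.
; A Follow timeline is wired to move and rotate the effect along the spline in local space, but nothing starts it.
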(event `self.ReceiveBeginPlay`
  (`KismetSystemLibrary.ExecuteConsoleCommand` "show splines" null))

(fn `UserConstructionScript`
  (`NiagaraComponent.SetVariableFloat` (`self.Niagara`) "UserSpawnRate" (`self.CustomSpawnRate`)))