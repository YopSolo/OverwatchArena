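; Base interactable actor that carries a configurable mesh and display name.
; The construction script adds a static mesh component and assigns it the StaticMesh variable.
; GetDisplayName returns the stored name, and the Interact event only prints it to screen behind a French "je s'appelle" (my name is) prefix, as placeholder behavior.
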(event `self.Interact`
  (bind _value (`self.getDisplayName`))
  (`KismetSystemLibrary.PrintString` (`KismetStringLibrary.Concat_StrStr` "je s'appelle : " (`KismetStringLibrary.Conv_NameToString` _value))))

(fn `getDisplayName`
  (returns (value :type Name))
  (return (`self.ActorDispayName`)))

(fn `UserConstructionScript`
  (bind _returnvalue (`AddComponent|NODE_AddStaticMeshComponent-0`))
  (`StaticMeshComponent.SetStaticMesh` _returnvalue (`self.StaticMesh`)))