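; BP_Mothership2 is an AI mothership that spawns BP_sentinel2 sentinels around itself.
; BeginPlay starts a looping timer, apparently driving SpawnSentinelle, which spawns one sentinel per call until a counter reaches its cap.
; Spawn locations are random points within half the SpawnhealZone box's X/Y extents, adjusted for collisions but always spawned.
; The counter is never decremented here, so destroyed sentinels are not replaced by this logic.
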(event `self.ReceiveBeginPlay`
  (`KismetSystemLibrary.K2_SetTimerDelegate` (`|CreateDelegate` :!event `Spawn Sentinelle`) 5.0 true))

(event `Spawn Sentinelle`
  (bind _spawn_heal_zone (`self.spawn/heal zone`))
  (bind (_returnvalue_x _returnvalue_y) (`KismetMathLibrary.BreakVector` (`SceneComponent.K2_GetComponentLocation` _spawn_heal_zone)))
  (bind (_returnvalue_x_2 _returnvalue_y_2) (`KismetMathLibrary.BreakVector` (`BoxComponent.GetScaledBoxExtent` _spawn_heal_zone)))
  (if (< (`self.sentinellesCounts`) 10.0)
    (bind _result (`/Engine/EditorBlueprintResources/StandardMacros.IncrementFloat` (`self.sentinellesCounts`))
      (:`  `
        (set `self.sentinellesCounts` _result)
        (`|SpawnActorFromClass` "/Game/AI/BP_sentinel2.BP_sentinel2_C" (`KismetMathLibrary.MakeTransform` (`KismetMathLibrary.RandomPointInBoundingBox` (`KismetMathLibrary.MakeVector` _returnvalue_x _returnvalue_y) (* (`KismetMathLibrary.MakeVector` _returnvalue_x_2 _returnvalue_y_2) 0.5))) "AdjustIfPossibleButAlwaysSpawn" "OverrideRootScale" null null)))))

(fn `UserConstructionScript`)