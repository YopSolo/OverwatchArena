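; BP_sentinel2 is a sentinel Blueprint in the AI folder whose only logic is a cosmetic animation, which nothing in the graph starts.
; The AnimPanels timeline would spin Shell in roll and yaw by frame delta time and pulse Panels' scale relative to Shell's, using a remapped sine.
; A FlipFlop on Finished would alternate forward and reverse playback to keep it looping.
; The construction script is empty.
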(fn `UserConstructionScript`)