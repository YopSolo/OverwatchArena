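; BP_LightGen is an interactable light prop, apparently a light generator, that toggles on and off each time it receives Interact.
; A FlipFlop alternates calls to SwitchLight, which shows or hides a SpotLight and four plane components together through their hidden-in-game state.
; The construction script runs the parent's script, then switches the light off, so it starts dark.
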(event `/Game/IInteractions/IInteractable.Interact`
  (`/Engine/EditorBlueprintResources/StandardMacros.FlipFlop`
    (:`A`
      (`self.SwitchLight` true))
    (:`B`
      (`self.SwitchLight` false))))

(fn `SwitchLight`
  (params (On :type Boolean))
  (bind _returnvalue (not On))
  (`SceneComponent.SetHiddenInGame` (`self.Plane1`) _returnvalue false)
  (`SceneComponent.SetHiddenInGame` (`self.Plane2`) _returnvalue false)
  (`SceneComponent.SetHiddenInGame` (`self.Plane3`) _returnvalue false)
  (`SceneComponent.SetHiddenInGame` (`self.Plane`) _returnvalue false)
  (`SceneComponent.SetHiddenInGame` (`self.SpotLight`) _returnvalue false))

(fn `UserConstructionScript`
  (`parent.UserConstructionScript`)
  (`self.SwitchLight` false))