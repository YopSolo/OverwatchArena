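; Quest-giver NPC with a floating quest marker and two stages of voiced dialogue.
; The first player character overlap with its box plays the intro dialogue and switches the marker text to a key prompt.
; The Talk event, called from outside, plays the second dialogue and hides the marker.
; Tick billboards the marker to the camera on the CPU (noted as inferior to a material), and mesh hover swaps the cursor to crosshairs.
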(event `self.StaticMesh.OnBeginCursorOver`
  (params (TouchedComponent :type "PrimitiveComponent Object Reference"))
  ;[0 0 0] Exemple de detection de curseur sur un elment 3d. Au préalable dans le player controller afficher la souris et activer le over event
  (set `PlayerController.CurrentMouseCursor` "Crosshairs" (`GameplayStatics.GetPlayerController` 0)))

(event `self.StaticMesh.OnEndCursorOver`
  (params (TouchedComponent :type "PrimitiveComponent Object Reference"))
  ;[0 0 0] Exemple de detection de curseur sur un elment 3d. Au préalable dans le player controller afficher la souris et activer le over event
  (set `PlayerController.CurrentMouseCursor` "Default" (`GameplayStatics.GetPlayerController` 0)))

(event `self.ReceiveTick`
  (params (DeltaSeconds :type "Float (single-precision)"))
  (bind (_returnvalue_roll _returnvalue_pitch _returnvalue_yaw) (`KismetMathLibrary.BreakRotator` (`PlayerCameraManager.GetCameraRotation` (`GameplayStatics.GetPlayerCameraManager` 0))))
  ;[0 0 0] !!! Vilain system de billboard (preferer un billboard material => GPU)
  (`SceneComponent.K2_SetWorldRotation` (`self.QuestMarker`) (`KismetMathLibrary.MakeRotator` _returnvalue_roll (* _returnvalue_pitch -1.0) (+ _returnvalue_yaw 180.0)) false false))

(event `self.Box.OnComponentBeginOverlap`
  (params (OverlappedComponent :type "PrimitiveComponent Object Reference") (OtherActor :type "Actor Object Reference") (OtherComp :type "PrimitiveComponent Object Reference") (OtherBodyIndex :type Integer) (bFromSweep :type Boolean) (SweepResult :type "HitResult Structure (by ref)"))
  ;[0 0 0] Trigger du systeme de dialogue
  (cast `/Game/OverwatchArena/BP/BP_OverwatchCharacter` OtherActor)
  (if (not (`self.IsQuestTriggered?`))
    (set `self.IsQuestTriggered?` true)
    (`GameplayStatics.PlayDialogue2D` "/Game/OverwatchArena/Quests/DW_Quest1.DW_Quest1" (make `DialogueContext` (`self.DialogVoiceNPC`) (`|MakeArray` "/Game/OverwatchArena/Quests/D_Player.D_Player" :!type "DialogueVoice Object Reference")) 0.0)
    (`TextRenderComponent.K2_SetText` (`self.QuestMarker`) "press (T)")))

(event `/Game/OverwatchArena/Quests/IQuestInterface.Talk`
  ;[0 0 0] Trigger du systeme de dialogue
  (`GameplayStatics.PlayDialogue2D` "/Game/OverwatchArena/Quests/DW_Quest2.DW_Quest2" (make `DialogueContext` (`self.DialogVoiceNPC`) (`|MakeArray` "/Game/OverwatchArena/Quests/D_Player.D_Player" :!type "DialogueVoice Object Reference")) 0.0)
  (`SceneComponent.SetHiddenInGame` (`self.QuestMarker`) true false))

(fn `UserConstructionScript`)