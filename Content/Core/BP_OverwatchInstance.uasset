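; Game instance that manages save slots, saving, restoring and deleting the player's saved transform.
; Init asynchronously loads the default slot into a cached BP_SaveGameObject, which SaveGame reuses, or replaces if the target slot is missing, before writing synchronously.
; LoadGame reads the slot directly without updating that cache, then teleports the player character and sets the controller's rotation.
; Save, load and delete print on-screen feedback in French, apart from "Load".
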(event `self.ReceiveInit`
  (bind (_savegame _bsuccess) (`AsyncActionHandleSaveGame.AsyncLoadGameFromSlot` (`self.defaultSaveSlotName`))
    (:`Completed`
      (if _bsuccess
        (bind _asbp_save_game_object (cast `/Game/Core/BP_SaveGameObject` _savegame))
        (set `self.mySaveGame` _asbp_save_game_object)))))

(fn `DeleteGameSlot`
  (params (SlotNameValue :type String))
  (bind _returnvalue (`GameplayStatics.DoesSaveGameExist` SlotNameValue))
  (if _returnvalue
    (bind _returnvalue_2 (`GameplayStatics.DeleteGameInSlot` (`local.SlotNameValue`)))
    (if _returnvalue_2
      (`KismetSystemLibrary.PrintString` (`KismetStringLibrary.Concat_StrStr` "slot " (`local.SlotNameValue`) " effacé") true false (struct :`R` 0.240366 :`G` 0.796875 :`B` 0.210332 :`A` 1.0)))
    (else
      (`KismetSystemLibrary.PrintString` "Pas de slot de sauvegarde a effacer" true false (struct :`R` 0.552011 :`G` 0.099899 :`B` 0.012287 :`A` 1.0)))))

(fn `LoadGame`
  (params (SlotNameValue :type String :default "defaultSlot"))
  (bind _returnvalue (`GameplayStatics.DoesSaveGameExist` SlotNameValue))
  (if _returnvalue
    (bind _returnvalue_2 (`GameplayStatics.LoadGameFromSlot` (`local.SlotNameValue`)))
    (`KismetSystemLibrary.PrintString` "Load" true false (struct :`R` 0.240366 :`G` 0.796875 :`B` 0.210332 :`A` 1.0))
    (bind _asbp_save_game_object (cast `/Game/Core/BP_SaveGameObject` _returnvalue_2))
    (bind (_myplayertransform_location _myplayertransform_rotation) (`KismetMathLibrary.BreakTransform` (`/Game/Core/BP_SaveGameObject.MyPlayerTransform` _asbp_save_game_object)))
    (`Controller.SetControlRotation` (`GameplayStatics.GetPlayerController` 0) _myplayertransform_rotation)
    (`Actor.K2_SetActorLocation` (`GameplayStatics.GetPlayerCharacter` 0) _myplayertransform_location false true)
    (else
      (`KismetSystemLibrary.PrintString` "Pas de slot de sauvegarde" true false (struct :`R` 0.552011 :`G` 0.099899 :`B` 0.012287 :`A` 1.0)))))

(fn `SaveGame`
  (params (SlotName :type String :default "defaultSlot") (MyPlayerTransformValue :type "Transform Structure"))
  (bind _returnvalue (`GameplayStatics.DoesSaveGameExist` SlotName))
  (if (not _returnvalue)
    ;[0 0 0] si le slot n'existe pas on le crée
    (bind _returnvalue_2 (`GameplayStatics.CreateSaveGameObject` "/Game/Core/BP_SaveGameObject.BP_SaveGameObject_C"))
    (set `self.mySaveGame` _returnvalue_2))
  ;[0 0 0] dès qu'on a le save game on sauve le transform
  (set `/Game/Core/BP_SaveGameObject.MyPlayerTransform` (`local.MyPlayerTransformValue`) (`self.mySaveGame`))
  ;[0 0 0] on ecrit la sauvegarde (fichier dans /save)
  (bind _returnvalue_3 (`GameplayStatics.SaveGameToSlot` (`self.mySaveGame`) (`local.SlotName`)))
  (if _returnvalue_3
    (`KismetSystemLibrary.PrintString` "Sauvegarde !" true false (struct :`R` 0.240366 :`G` 0.796875 :`B` 0.210332 :`A` 1.0))))